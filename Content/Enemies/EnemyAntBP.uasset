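; Ant enemy that moves toward the player pawn, fires at actors in its detection radius and self-destructs to damage the player.
; Movement sets BaseReached on arrival, switching off timer-throttled projectile fire at every overlapping actor and enabling the close-range attack.
; The behaviour events have no callers here, as Tick and BeginPlay are empty.
; EndPlay spawns a death effect and awards points to the first-person character, whatever the cause of removal.
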(event Custom|CustomEvent
  (Variables|Default|SetCanFire true))

(event EventBeginPlay)

(event EventEndPlay
  (params (EndPlayReason :type EEndPlayReason%20Enum :default "Destroyed"))
  (Niagara|SpawnSystematLocation "/Game/EnemyDeath.EnemyDeath" (+ (Transformation|GetActorLocation) "0.000000,0.000000,100.000000"))
  (bind _asbp_first_person_character (Utilities|Casting|CastToBP_FirstPersonCharacter (Game|Player|GetPlayerPawn 0)))
  (Variables|/Game/FirstPerson/Blueprints/BP_FirstPersonCharacter.BP_FirstPersonCharacter_C|SetPoints _asbp_first_person_character (+ (Variables|/Game/FirstPerson/Blueprints/BP_FirstPersonCharacter.BP_FirstPersonCharacter_C|GetPoints _asbp_first_person_character) 2)))

(event EventTick
  (params (DeltaSeconds :type Float%20%28single-precision%29)))

(event Collision|EventActorBeginOverlap
  (params (OtherActor :type Actor%20Object%20Reference)))

(event EventEnemyCloseBehaviour
  (bind _returnvalue (Game|Player|GetPlayerPawn 0))
  (if (Variables|Default|GetBaseReached)
    (Utilities|IsValid _returnvalue
      (:Is%20Valid
        (if (Collision|IsOverlappingActor (Variables|Default|GetTowerDetectionRadius) _returnvalue :!class /Script/Engine.PrimitiveComponent)
          (Game|Damage|ApplyDamage _returnvalue 5.0 0 self)
          (Actor|DestroyActor))))))

(event EventEnemyMovementBehaviour
  (bind _returnvalue (Game|Player|GetPlayerPawn 0))
  (Utilities|IsValid _returnvalue
    (:Is%20Valid
      (AI|AIMoveTo self (Transformation|GetActorLocation _returnvalue) 0 3e+01 false
        (:OnSuccess
          (Variables|Default|SetBaseReached true))))))

(event EventEnemyRangedBehaviour
  (bind _projpos (Variables|Default|GetProjPos))
  (bind _returnvalue (Transformation|GetWorldLocation _projpos))
  (if (not (Variables|Default|GetBaseReached))
    (if (Variables|Default|GetCanFire)
      (Variables|Default|SetCanFire false)
      (for _array_element (Collision|GetOverlappingActors (Variables|Default|GetTowerDetectionRadius) 0 :!class /Script/Engine.PrimitiveComponent)
        (Game|SpawnActorfromClass "/Game/Enemies/EnemyProjectileBP.EnemyProjectileBP_C" (Math|Transform|MakeTransform _returnvalue (Math|Rotator|FindLookatRotation _returnvalue (Transformation|GetActorLocation _array_element))) "AlwaysSpawn" "MultiplyWithRoot" 0 0))
      (Utilities|Time|SetTimerbyEvent (delegate Custom|CustomEvent) 1.0))))

(fn ConstructionScript)