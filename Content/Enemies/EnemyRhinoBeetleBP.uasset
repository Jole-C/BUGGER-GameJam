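; Rhino beetle enemy that walks toward the player and self-destructs as an area attack.
; Movement behaviour uses AIMoveTo on the player pawn's current location, flagging BaseReached on arrival within acceptance range.
; Close behaviour then starts a one-shot fuse that damages every other actor overlapping TowerDetectionRadius and destroys the beetle.
; EndPlay spawns a heavy death effect and awards player points, so self-detonation scores too.
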(event Custom|CustomEvent
  (bind _self self)
  (for _array_element (Collision|GetOverlappingActors (Variables|Default|GetTowerDetectionRadius) 0 :!class /Script/Engine.PrimitiveComponent)
    (if (!= _array_element _self)
      (Game|Damage|ApplyDamage _array_element 4e+01 0 _self)))
  (Actor|DestroyActor))

(event EventBeginPlay)

(event EventEndPlay
  (params (EndPlayReason :type EEndPlayReason%20Enum :default "Destroyed"))
  (Niagara|SpawnSystematLocation "/Game/EnemyDeathHeavy.EnemyDeathHeavy" (+ (Transformation|GetActorLocation) "0.000000,0.000000,100.000000"))
  (bind _asbp_first_person_character (Utilities|Casting|CastToBP_FirstPersonCharacter (Game|Player|GetPlayerPawn 0)))
  (Variables|/Game/FirstPerson/Blueprints/BP_FirstPersonCharacter.BP_FirstPersonCharacter_C|SetPoints _asbp_first_person_character (+ (Variables|/Game/FirstPerson/Blueprints/BP_FirstPersonCharacter.BP_FirstPersonCharacter_C|GetPoints _asbp_first_person_character) 100)))

(event EventTick
  (params (DeltaSeconds :type Float%20%28single-precision%29)))

(event Collision|EventActorBeginOverlap
  (params (OtherActor :type Actor%20Object%20Reference)))

(event EventEnemyCloseBehaviour
  (if (Variables|Default|GetBaseReached)
    (if (not (Variables|Default|GetPlayerReached))
      (Variables|Default|SetPlayerReached true)
      (Utilities|Time|SetTimerbyEvent (delegate Custom|CustomEvent) 3.0))))

(event EventEnemyMovementBehaviour
  (bind _returnvalue (Game|Player|GetPlayerPawn 0))
  (if (not (Variables|Default|GetBaseReached))
    (Utilities|IsValid _returnvalue
      (:Is%20Valid
        (AI|AIMoveTo self (Transformation|GetActorLocation _returnvalue) 0 3.5e+02 false
          (:OnSuccess
            (Variables|Default|SetBaseReached true)))))))

(fn ConstructionScript)