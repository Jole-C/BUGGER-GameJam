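; Centipede enemy body segment that trails its Follower actor and attacks from range.
; The movement event uses AI MoveTo toward the Follower, while the ranged event damages a random actor overlapping TowerDetectionRadius, gated by a timer cooldown.
; The validity check and damage call each make a separate random pick.
; EndPlay spawns a death effect and awards points to the player character, whatever the reason for removal.
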(event Custom|CustomEvent
  (Variables|Default|SetCanFire true))

(event EventBeginPlay)

(event EventEndPlay
  (params (EndPlayReason :type EEndPlayReason%20Enum :default "Destroyed"))
  (Niagara|SpawnSystematLocation "/Game/EnemyDeath.EnemyDeath" (+ (Transformation|GetActorLocation) "0.000000,0.000000,100.000000"))
  (bind _asbp_first_person_character (Utilities|Casting|CastToBP_FirstPersonCharacter (Game|Player|GetPlayerPawn 0)))
  (Variables|/Game/FirstPerson/Blueprints/BP_FirstPersonCharacter.BP_FirstPersonCharacter_C|SetPoints _asbp_first_person_character (+ (Variables|/Game/FirstPerson/Blueprints/BP_FirstPersonCharacter.BP_FirstPersonCharacter_C|GetPoints _asbp_first_person_character) 5)))

(event EventTick
  (params (DeltaSeconds :type Float%20%28single-precision%29)))

(event EventEnemyMovementBehaviour
  (bind _follower (Variables|Default|GetFollower))
  (Utilities|IsValid _follower
    (:Is%20Valid
      (AI|AIMoveTo self (Transformation|GetActorLocation _follower) 0 1.2e+02 false))))

(event EventEnemyRangedBehaviour
  (bind _towerdetectionradius (Variables|Default|GetTowerDetectionRadius))
  (bind _overlappingactors (Collision|GetOverlappingActors _towerdetectionradius 0 :!class /Script/Engine.PrimitiveComponent))
  (bind _outitem (Utilities|Array|Random _overlappingactors))
  (if (Variables|Default|GetCanFire)
    (Utilities|IsValid _outitem
      (:Is%20Valid
        (Variables|Default|SetCanFire false)
        (Game|Damage|ApplyDamage _outitem 2.0 0 0)
        (Utilities|Time|SetTimerbyEvent (delegate Custom|CustomEvent) 3.0)))))

(event Collision|EventActorBeginOverlap
  (params (OtherActor :type Actor%20Object%20Reference)))

(fn ConstructionScript)