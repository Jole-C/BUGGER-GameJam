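; Test tower actor that shoots projectiles at enemies in its overlap list.
; TowerBehaviour, not called within this file, clears CanFire and spawns a ShootTowerProjectileBP at ProjectilePos, rotated toward a random entry from OverlappingEnemies.
; A one-shot reload timer restores CanFire, but only starts after a shot, so an invalid pick leaves firing disabled.
; The random pick is a pure node, so the validated enemy can differ from the aimed one.
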(event Custom|CustomEvent
  (Variables|Default|SetCanFire true))

(event EventBeginPlay)

(event Collision|EventActorBeginOverlap
  (params (OtherActor :type Actor%20Object%20Reference)))

(event EventTick
  (params (DeltaSeconds :type Float%20%28single-precision%29)))

(event EventTowerBehaviour
  (bind _overlappingenemies (Variables|Default|GetOverlappingEnemies))
  (bind _projectilepos (Variables|Default|GetProjectilePos))
  (bind _outitem (Utilities|Array|Random _overlappingenemies))
  (bind _returnvalue (Transformation|GetWorldLocation _projectilepos))
  (if (Variables|Default|GetCanFire)
    (Variables|Default|SetCanFire false)
    (Utilities|IsValid _outitem
      (:Is%20Valid
        (Game|SpawnActorfromClass "/Game/Towers/ShootTowerProjectileBP.ShootTowerProjectileBP_C" (Math|Transform|MakeTransform _returnvalue (Math|Rotator|FindLookatRotation _returnvalue (Transformation|GetActorLocation _outitem))) "AlwaysSpawn" "MultiplyWithRoot" 0 0)
        (Utilities|Time|SetTimerbyEvent (delegate Custom|CustomEvent) (Variables|Default|GetShootReloadTime))))))

(fn ConstructionScript)