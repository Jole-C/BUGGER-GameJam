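; Melee tower that deals area damage, hitting every valid enemy in its overlap list at once.
; TowerBehaviour clears CanFire, then applies damage and spawns a small EnemyDeath Niagara effect on each enemy, whether or not it dies.
; An AttackSpeed timer restores CanFire, but it is set inside the loop, so an attack with no valid enemies leaves CanFire false.
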(event Custom|CustomEvent
  (Variables|Default|SetCanFire true))

(event EventBeginPlay)

(event Collision|EventActorBeginOverlap
  (params (OtherActor :type Actor%20Object%20Reference)))

(event EventTick
  (params (DeltaSeconds :type Float%20%28single-precision%29)))

(event EventTowerBehaviour
  (if (Variables|Default|GetCanFire)
    (Variables|Default|SetCanFire false)
    (for _array_element (Variables|Default|GetOverlappingEnemies)
      (Utilities|IsValid _array_element
        (:Is%20Valid
          (Niagara|SpawnSystematLocation "/Game/EnemyDeath.EnemyDeath" (Transformation|GetActorLocation _array_element) "0, 0, 0" "0.025000,0.025000,0.025000")
          (Game|Damage|ApplyDamage _array_element (Variables|Default|GetDamage) 0 self)
          (Utilities|Time|SetTimerbyEvent (delegate Custom|CustomEvent) (Variables|Default|GetAttackSpeed)))))))

(fn ConstructionScript)